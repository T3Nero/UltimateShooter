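; Player HUD for the shooter that draws a dynamic four-piece crosshair slightly above screen centre.
; BeginPlay caches the player pawn as BP_ShooterCharacter.
; Each DrawHUD reads that character's crosshair spread multiplier and offsets the top, bottom, left and right quad textures outward from the crosshair centre, scaled by a maximum spread value.
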(event EventBeginPlay
  (bind _asbp_shooter_character (Utilities|Casting|CastToBP_ShooterCharacter (Game|Player|GetPlayerPawn 0)))
  (Variables|Default|SetAs%20BP%20Shooter%20Character _asbp_shooter_character))

(event EventDrawHUD
  (params (SizeX :type Integer) (SizeY :type Integer))
  (bind _as_bp_shooter_character (Variables|Default|GetAs%20BP%20Shooter%20Character))
  (Variables|Default|SetScreenCentre (Math|Vector2D|MakeVector2D (Math|Conversions|ToFloat(Integer) (/ SizeX 2)) (Math|Conversions|ToFloat(Integer) (/ SizeY 2))))
  (Variables|Default|SetCrosshairLocation (Math|Vector2D|MakeVector2D (.X (Math|Vector2D|BreakVector2D (Variables|Default|GetScreenCentre))) (- (.Y (Math|Vector2D|BreakVector2D (Variables|Default|GetScreenCentre))) 5e+01)))
  (Utilities|IsValid _as_bp_shooter_character
    (:Is%20Valid
      (Variables|Default|SetCrosshairSpreadMultiplier (Class|ParentCharacter|GetCrosshairSpreadMultiplier _as_bp_shooter_character))
      ;[1 1 1] Centre of crosshair location
      (Variables|Default|SetCrosshairBaseCentre (Math|Vector2D|MakeVector2D (- (.X (Math|Vector2D|BreakVector2D (Variables|Default|GetCrosshairLocation))) (Variables|Default|GetCrosshairHalfWidth)) (- (.Y (Math|Vector2D|BreakVector2D (Variables|Default|GetCrosshairLocation))) (Variables|Default|GetCrosshairHalfHeight))))
      (Canvas|DrawTexture "/Game/_Assets/Textures/Crosshairs/Crosshair_Quad_9_Bottom.Crosshair_Quad_9_Bottom" (.X (Math|Vector2D|BreakVector2D (Variables|Default|GetCrosshairBaseCentre))) (+ (.Y (Math|Vector2D|BreakVector2D (Variables|Default|GetCrosshairBaseCentre))) (* (Variables|Default|GetCrosshairSpreadMultiplier) (Variables|Default|GetCrosshairSpreadMax))) 64.0 64.0 0.0 0.0 1.0 1.0 "(R=1.000000,G=1.000000,B=1.000000,A=1.000000)")
      (Canvas|DrawTexture "/Game/_Assets/Textures/Crosshairs/Crosshair_Quad_9_Top.Crosshair_Quad_9_Top" (.X (Math|Vector2D|BreakVector2D (Variables|Default|GetCrosshairBaseCentre))) (- (.Y (Math|Vector2D|BreakVector2D (Variables|Default|GetCrosshairBaseCentre))) (* (Variables|Default|GetCrosshairSpreadMultiplier) (Variables|Default|GetCrosshairSpreadMax))) 64.0 64.0 0.0 0.0 1.0 1.0 "(R=1.000000,G=1.000000,B=1.000000,A=1.000000)")
      (Canvas|DrawTexture "/Game/_Assets/Textures/Crosshairs/Crosshair_Quad_9_Left.Crosshair_Quad_9_Left" (- (.X (Math|Vector2D|BreakVector2D (Variables|Default|GetCrosshairBaseCentre))) (* (Variables|Default|GetCrosshairSpreadMultiplier) (Variables|Default|GetCrosshairSpreadMax))) (.Y (Math|Vector2D|BreakVector2D (Variables|Default|GetCrosshairBaseCentre))) 64.0 64.0 0.0 0.0 1.0 1.0 "(R=1.000000,G=1.000000,B=1.000000,A=1.000000)")
      (Canvas|DrawTexture "/Game/_Assets/Textures/Crosshairs/Crosshair_Quad_9_Right.Crosshair_Quad_9_Right" (+ (.X (Math|Vector2D|BreakVector2D (Variables|Default|GetCrosshairBaseCentre))) (* (Variables|Default|GetCrosshairSpreadMultiplier) (Variables|Default|GetCrosshairSpreadMax))) (.Y (Math|Vector2D|BreakVector2D (Variables|Default|GetCrosshairBaseCentre))) 64.0 64.0 0.0 0.0 1.0 1.0 "(R=1.000000,G=1.000000,B=1.000000,A=1.000000)"))))

(fn ConstructionScript)